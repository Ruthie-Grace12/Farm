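; BP_FunctionalityCore is the settings backend for the InfectionUI options menu, covering video, audio and game options.
; One dispatcher switches on a setting type, passes an option index or float to that setting's function, and returns a display label for indexed options.
; Setters use GameUserSettings, console commands, sound mix class overrides, culture switching or the game instance's tutorial flag.
; It never applies or saves GameUserSettings itself, but supplies save slot names.
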(fn WhatFunctionalityDoYouWant?
  (params (WhatFunctionality? :type E_Functionality%20Enum :default "NewEnumerator0") (IntValue :type Integer) (FloatValue :type Float%20%28double-precision%29))
  (switch Utilities|FlowControl|Switch|SwitchonE_Functionality WhatFunctionality?
    (:NewEnumerator0
      (bind _displaymodetext (Functions|Video|DisplayMode IntValue))
      (LocalVariables|SetText _displaymodetext))
    (:NewEnumerator1
      (bind _vsynctext (Functions|Video|VSync IntValue))
      (LocalVariables|SetText _vsynctext))
    (:NewEnumerator2
      (bind _motionblurtext (Functions|Video|MotionBlur IntValue))
      (LocalVariables|SetText _motionblurtext))
    (:NewEnumerator3
      (bind _aatext (Functions|Video|Antialiasing IntValue))
      (LocalVariables|SetText _aatext))
    (:NewEnumerator9
      (bind _lodtext (Functions|Video|LevelOfDetail IntValue))
      (LocalVariables|SetText _lodtext))
    (:NewEnumerator4
      (bind _texturestext (Functions|Video|TexturesQuality IntValue))
      (LocalVariables|SetText _texturestext))
    (:NewEnumerator5
      (bind _shadowtext (Functions|Video|ShadowQuality IntValue))
      (LocalVariables|SetText _shadowtext))
    (:NewEnumerator6
      (bind _overalltext (Functions|Video|OverallQuality IntValue))
      (LocalVariables|SetText _overalltext))
    (:NewEnumerator7
      (Functions|Audio|AudioMusic FloatValue))
    (:NewEnumerator8
      (Functions|Audio|AudioFX FloatValue))
    (:NewEnumerator10
      (bind _showtutorialtext (Functions|Game|ShowTutorials IntValue))
      (LocalVariables|SetText _showtutorialtext))
    (:NewEnumerator11
      (bind _subtitlestext (Functions|Game|Subtitles IntValue))
      (LocalVariables|SetText _subtitlestext))
    (:NewEnumerator12
      (bind _languagestext (Functions|Game|Languages IntValue))
      (LocalVariables|SetText _languagestext))
    (:NewEnumerator13
      (bind _hdrtext (Functions|Game|HDR IntValue))
      (LocalVariables|SetText _hdrtext))
    (:NewEnumerator14
      (Functions|Game|Gamma FloatValue)))
  (return (LocalVariables|GetText)))

(fn DisplayMode
  (params (Options :type Integer))
  (bind _returnvalue (Settings|GetGameUserSettings))
  (Class|GameUserSettings|SetFullscreenMode _returnvalue (Utilities|Select :Index Options :Option%200 "Windowed" :Option%201 "WindowedFullscreen" :Option%202 "Fullscreen"))
  (return Options (Utilities|Select :Index Options :Option%200 "WINDOWED" :Option%201 "BORDERLESS" :Option%202 "FULLSCREEN")))

(fn VSync
  (params (Options :type Integer))
  (bind _returnvalue (Settings|GetGameUserSettings))
  (Class|GameUserSettings|SetVSyncEnabled _returnvalue (Utilities|Select :Index Options :Option%200 false :Option%201 true))
  (return Options (Utilities|Select :Index Options :Option%200 "OFF" :Option%201 "ON")))

(fn MotionBlur
  (params (Options :type Integer))
  (Development|ExecuteConsoleCommand 0 (Utilities|String|Append "r.DefaultFeature.MotionBlur " (Utilities|Select :Index Options :Option%200 "0" :Option%201 "1")) 0)
  (return Options (Utilities|Select :Index Options :Option%200 "OFF" :Option%201 "ON")))

(fn Antialiasing
  (params (Options :type Integer))
  (bind _returnvalue (Settings|GetGameUserSettings))
  (Class|GameUserSettings|SetAntiAliasingQuality _returnvalue (Utilities|Select :Index Options :Option%200 0 :Option%201 4))
  (Development|ExecuteConsoleCommand 0 (Utilities|String|Append " r.TemporalAA.Upsampling " (Utilities|Select :Index Options :Option%200 "0" :Option%201 "1")) 0)
  (return Options (Utilities|Select :Index Options :Option%200 "OFF" :Option%201 "ON")))

(fn LevelOfDetail
  (params (Options :type Integer))
  (bind _returnvalue (Utilities|Select :Index Options :Option%200 2 :Option%201 1 :Option%202 0))
  (bind _returnvalue_2 (Utilities|String|ToString(Integer) _returnvalue))
  (bind _returnvalue_3 (Settings|GetGameUserSettings))
  (Class|GameUserSettings|SetViewDistanceQuality _returnvalue_3 Options)
  (Development|ExecuteConsoleCommand 0 (Utilities|String|Append "r.ForceLOD " _returnvalue_2) 0 :!pinned true) ; 0: LOD Max; 2:LOD Min
  (Development|ExecuteConsoleCommand 0 (Utilities|String|Append "r.SkeletalMeshLODBias " _returnvalue_2) 0)
  (return Options (Utilities|Select :Index Options :Option%200 "LOW" :Option%201 "MEDIUM" :Option%202 "HIGH")))

(fn TexturesQuality
  (params (Options :type Integer))
  (bind _returnvalue (Settings|GetGameUserSettings))
  (Class|GameUserSettings|SetTextureQuality _returnvalue (Utilities|Select :Index Options :Option%200 0 :Option%201 1 :Option%202 2 :Option%203 3 :Option%204 4))
  (return Options (Utilities|Select :Index Options :Option%200 "LOW" :Option%201 "MEDIUM" :Option%202 "HIGH" :Option%203 "ULTRA" :Option%204 "MAX")))

(fn ShadowQuality
  (params (Options :type Integer))
  (bind _returnvalue (Settings|GetGameUserSettings))
  (Class|GameUserSettings|SetShadowQuality _returnvalue (Utilities|Select :Index Options :Option%200 0 :Option%201 1 :Option%202 2 :Option%203 3 :Option%204 4))
  (return Options (Utilities|Select :Index Options :Option%200 "NONE" :Option%201 "MEDIUM" :Option%202 "HIGH" :Option%203 "ULTRA" :Option%204 "MAX")))

(fn OverallQuality
  (params (Options :type Integer))
  (bind _returnvalue (Utilities|Select :Index Options :Option%200 0 :Option%201 1 :Option%202 2 :Option%203 3 :Option%204 4))
  (bind _returnvalue_2 (Settings|GetGameUserSettings))
  (Class|GameUserSettings|SetPostProcessingQuality _returnvalue_2 _returnvalue)
  (Class|GameUserSettings|SetVisualEffectQuality _returnvalue_2 _returnvalue)
  (Class|GameUserSettings|SetFoliageQuality _returnvalue_2 _returnvalue)
  (return Options (Utilities|Select :Index Options :Option%200 "LOW" :Option%201 "MEDIUM" :Option%202 "HIGH" :Option%203 "ULTRA" :Option%204 "MAX")))

(fn AudioFX
  (params (Volume :type Float%20%28double-precision%29))
  (Audio|SetSoundMixClassOverride 0 "/Game/InfectionUI/Audio/MySoundMix.MySoundMix" "/Game/InfectionUI/Audio/SoundClass_FX.SoundClass_FX" Volume 1.0 1.0 false)
  (Audio|PushSoundMixModifier 0 "/Game/InfectionUI/Audio/MySoundMix.MySoundMix"))

(fn AudioMusic
  (params (Volume :type Float%20%28double-precision%29))
  (Audio|SetSoundMixClassOverride 0 "/Game/InfectionUI/Audio/MySoundMix.MySoundMix" "/Game/InfectionUI/Audio/SoundClass_Music.SoundClass_Music" Volume 1.0 1.0 false)
  (Audio|PushSoundMixModifier 0 "/Game/InfectionUI/Audio/MySoundMix.MySoundMix"))

(fn ShowTutorials
  (params (Options :type Integer))
  (Variables|/Game/InfectionUI/Blueprints/BP_Infection_GI.BP_Infection_GI_C|SetShowTutorial (CallFunction|MyGetGameInstance) (Utilities|Select :Index Options :Option%200 false :Option%201 true))
  (return Options (Utilities|Select :Index Options :Option%200 "OFF" :Option%201 "ON")))

(fn MyGetGameInstance
  (bind _asbp_infection_gi (Utilities|Casting|CastToBP_Infection_GI (Game|GetGameInstance)))
  (return _asbp_infection_gi))

(fn Subtitles
  (params (Options :type Integer))
  (Class|GameplayStatics|SetSubtitlesEnabled (Utilities|Select :Index Options :Option%200 false :Option%201 true))
  (return Options (Utilities|Select :Index Options :Option%200 "OFF" :Option%201 "ON")))

(fn Languages
  (params (Options :type Integer))
  (Class|KismetInternationalizationLibrary|SetCurrentLanguageandLocale (Utilities|Select :Index Options :Option%200 "en" :Option%201 "es" :Option%202 "fr" :Option%203 "de" :Option%204 "it" :Option%205 "pt-BR" :Option%206 "pt-PT" :Option%207 "ru" :Option%208 "el" :Option%209 "ja"))
  (return Options (Utilities|Select :Index Options :Option%200 "ENGLISH" :Option%201 "SPANISH" :Option%202 "FRENCH" :Option%203 "GERMAN" :Option%204 "ITALIAN" :Option%205 "PORTUGUESE(BR)" :Option%206 "PORTUGUESE(PT)" :Option%207 "RUSSIAN" :Option%208 "GREEK" :Option%209 "JAPANESE")))

(fn HDR
  (params (Options :type Integer))
  (bind _returnvalue (Settings|GetGameUserSettings))
  (Class|GameUserSettings|EnableHDRDisplayOutput _returnvalue (Utilities|Select :Index Options :Option%200 false :Option%201 true) 1000)
  (return Options (Utilities|Select :Index Options :Option%200 "OFF" :Option%201 "ON")))

(fn Gamma
  (params (Value :type Float%20%28double-precision%29))
  (Development|ExecuteConsoleCommand 0 (Utilities|String|Append "gamma " (Utilities|String|ToString(Float) (* (Math|Float|MapRangeClamped Value 0.0 1.0 0.0 1.0) 5.0))) 0))

(fn MySaveGameSlot
  (params (GameSlot :type E_GameSlot%20Enum :default "NewEnumerator0"))
  (return (Utilities|Select :Index GameSlot :NewEnumerator0 "infection/video" :NewEnumerator1 "infection/audio" :NewEnumerator2 "infection/game")))

(fn MyRandomFloat
  (return (Math|Random|RandomFloatinRange 7.5e+02 1e+03)))