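; Master camera for the front-end menus, flying a cine camera between the title screen, main menu and its sub-screens.
; On BeginPlay it registers with the game instance, shows WBP_Infection and binds a timeline move that opens WBP_MainMenu.
; MoveMasterCamera lerps one location and one rotation axis per menu option, then spawns that option's widget.
; ReturntoMainMenu runs similar per-option lerps on its own timeline without creating a widget.
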(event Custom|MoveCameraToMainMenu
  (bind _cinecamera (Variables|Default|GetCineCamera))
  (bind _returnvalue (Transformation|GetWorldLocation _cinecamera))
  (bind _returnvalue_2 (Transformation|GetWorldRotation _cinecamera))
  ;[1 1 1] Here you set the camera on the map, load the title UI,
  ; move the camera forward to show the Main Menu UI.
  (bind _moving (Timeline|TL_MoveToMainMenu Play)
    (:Update
      (Transformation|SetWorldLocationAndRotation _cinecamera (Math|Vector|MakeVector (.x _returnvalue) (Math|Float|Lerp (.y _returnvalue) 4.5e+02 _moving) (.z _returnvalue)) (Math|Rotator|MakeRotator (.roll _returnvalue_2) (.pitch _returnvalue_2) (Math|Float|Lerp (.yaw _returnvalue_2) -83.0 _moving)) false false))
    (:Finished
      (bind _returnvalue_3 (UserInterface|CreateWidget "/Game/InfectionUI/UI/WBP_MainMenu.WBP_MainMenu_C" 0 self))
      (UserInterface|Viewport|AddtoViewport _returnvalue_3 0))))

(event EventBeginPlay
  ;[1 1 1] Here you set the camera on the map, load the title UI,
  ; move the camera forward to show the Main Menu UI.
  (Utilities|FlowControl|Sequence
    (:then_0
      (Variables|/Game/InfectionUI/Blueprints/BP_Infection_GI.BP_Infection_GI_C|SetMasterCamera (CallFunction|MyGetGameInstance) self))
    (:then_1
      (bind _returnvalue (UserInterface|CreateWidget "/Game/InfectionUI/UI/WBP_Infection.WBP_Infection_C"))
      (Variables|Default|SetUI_InfectionRef _returnvalue)
      (UserInterface|Viewport|AddtoViewport _returnvalue 0))
    (:then_2
      (EventDispatchers|BindEventtoMoveCameratoMainMenu (Variables|Default|GetUI_InfectionRef) (delegate Custom|MoveCameraToMainMenu)))))

(event EventMoveMasterCamera
  (params (Location :type Float%20%28double-precision%29) (Rotation :type Float%20%28double-precision%29) (OptionFromMenu :type E_MainMenuOptions%20Enum :default "NewEnumerator0"))
  (bind _cinecamera (Variables|Default|GetCineCamera))
  (bind _cinecamera_2 (Variables|Default|GetCineCamera))
  (bind _cinecamera_3 (Variables|Default|GetCineCamera))
  (bind _cinecamera_4 (Variables|Default|GetCineCamera))
  (bind _cinecamera_5 (Variables|Default|GetCineCamera))
  (bind _cinecamera_6 (Variables|Default|GetCineCamera))
  (bind _returnvalue (Transformation|GetWorldLocation _cinecamera))
  (bind _returnvalue_2 (Transformation|GetWorldRotation _cinecamera))
  (bind _returnvalue_3 (Transformation|GetWorldLocation _cinecamera_2))
  (bind _returnvalue_4 (Transformation|GetWorldRotation _cinecamera_2))
  (bind _returnvalue_5 (Transformation|GetWorldLocation _cinecamera_3))
  (bind _returnvalue_6 (Transformation|GetWorldRotation _cinecamera_3))
  (bind _returnvalue_7 (Transformation|GetWorldLocation _cinecamera_4))
  (bind _returnvalue_8 (Transformation|GetWorldRotation _cinecamera_4))
  (bind _returnvalue_9 (Transformation|GetWorldLocation _cinecamera_5))
  (bind _returnvalue_10 (Transformation|GetWorldRotation _cinecamera_5))
  (bind _returnvalue_11 (Transformation|GetWorldLocation _cinecamera_6))
  (bind _returnvalue_12 (Transformation|GetWorldRotation _cinecamera_6))
  (bind _moving (Timeline|MasterCamMove PlayFromStart)
    (:Update
      (switch Utilities|FlowControl|Switch|SwitchonE_MainMenuOptions OptionFromMenu
        (:NewEnumerator0
          (Transformation|SetWorldLocationAndRotation _cinecamera_6 (Math|Vector|MakeVector (.x _returnvalue_11) (.y _returnvalue_11) (Math|Float|Lerp (.z _returnvalue_11) Location _moving)) (Math|Rotator|MakeRotator (.roll _returnvalue_12) (Math|Float|Lerp (.pitch _returnvalue_12) Rotation _moving) (.yaw _returnvalue_12)) false false :!pinned true) ; Play
        )
        (:NewEnumerator1
          (Transformation|SetWorldLocationAndRotation _cinecamera_3 (Math|Vector|MakeVector (Math|Float|Lerp (.x _returnvalue_5) Location _moving) (.y _returnvalue_5) (.z _returnvalue_5)) (Math|Rotator|MakeRotator (.roll _returnvalue_6) (.pitch _returnvalue_6) (Math|Float|Lerp (.yaw _returnvalue_6) Rotation _moving)) false false :!pinned true) ; Game
        )
        (:NewEnumerator2
          (Transformation|SetWorldLocationAndRotation _cinecamera (Math|Vector|MakeVector (Math|Float|Lerp (.x _returnvalue) Location _moving) (.y _returnvalue) (.z _returnvalue)) (Math|Rotator|MakeRotator (.roll _returnvalue_2) (.pitch _returnvalue_2) (Math|Float|Lerp (.yaw _returnvalue_2) Rotation _moving)) false false :!pinned true) ; Video
        )
        (:NewEnumerator3
          (Transformation|SetWorldLocationAndRotation _cinecamera_2 (Math|Vector|MakeVector (.x _returnvalue_3) (.y _returnvalue_3) (Math|Float|Lerp (.z _returnvalue_3) Location _moving)) (Math|Rotator|MakeRotator (Math|Float|Lerp (.roll _returnvalue_4) 0.0 _moving) (.pitch _returnvalue_4) (.yaw _returnvalue_4)) false false :!pinned true) ; Audio
        )
        (:NewEnumerator5
          (Transformation|SetWorldLocationAndRotation _cinecamera_5 (Math|Vector|MakeVector (.x _returnvalue_9) (.y _returnvalue_9) (Math|Float|Lerp (.z _returnvalue_9) Location _moving)) (Math|Rotator|MakeRotator (.roll _returnvalue_10) (.pitch _returnvalue_10) (Math|Float|Lerp (.yaw _returnvalue_10) Rotation _moving)) false false :!pinned true) ; Extras
        )
        (:NewEnumerator6
          (Transformation|SetWorldLocationAndRotation _cinecamera_4 (Math|Vector|MakeVector (Math|Float|Lerp (.x _returnvalue_7) Location _moving) (.y _returnvalue_7) (.z _returnvalue_7)) (Math|Rotator|MakeRotator (.roll _returnvalue_8) (.pitch _returnvalue_8) (Math|Float|Lerp (.yaw _returnvalue_8) Rotation _moving)) false false :!pinned true) ; Exit
        )))
    (:Finished
      (bind _returnvalue_13 (UserInterface|CreateWidget (Utilities|Select :Index OptionFromMenu :NewEnumerator0 "/Game/InfectionUI/UI/WBP_ChoiceDifficulty.WBP_ChoiceDifficulty_C" :NewEnumerator1 "/Game/InfectionUI/UI/Menus/WBP_GameSettings.WBP_GameSettings_C" :NewEnumerator2 "/Game/InfectionUI/UI/Menus/WBP_VideoSettings.WBP_VideoSettings_C" :NewEnumerator3 "/Game/InfectionUI/UI/Menus/WBP_AudioSettings.WBP_AudioSettings_C" :NewEnumerator5 "/Game/InfectionUI/UI/Menus/WBP_Extras.WBP_Extras_C" :NewEnumerator6 "/Game/InfectionUI/UI/Menus/WBP_Exit.WBP_Exit_C")))
      (UserInterface|Viewport|AddtoViewport _returnvalue_13 0))))

(event EventReturntoMainMenu
  (params (ReturnMainMenu :type E_MainMenuOptions%20Enum :default "NewEnumerator0") (Location :type Float%20%28double-precision%29) (Rotation :type Float%20%28double-precision%29))
  (bind _cinecamera (Variables|Default|GetCineCamera))
  (bind _cinecamera_2 (Variables|Default|GetCineCamera))
  (bind _cinecamera_3 (Variables|Default|GetCineCamera))
  (bind _cinecamera_4 (Variables|Default|GetCineCamera))
  (bind _cinecamera_5 (Variables|Default|GetCineCamera))
  (bind _cinecamera_6 (Variables|Default|GetCineCamera))
  (bind _returnvalue (Transformation|GetWorldLocation _cinecamera))
  (bind _returnvalue_2 (Transformation|GetWorldRotation _cinecamera))
  (bind _returnvalue_3 (Transformation|GetWorldLocation _cinecamera_2))
  (bind _returnvalue_4 (Transformation|GetWorldRotation _cinecamera_2))
  (bind _returnvalue_5 (Transformation|GetWorldLocation _cinecamera_4))
  (bind _returnvalue_6 (Transformation|GetWorldRotation _cinecamera_4))
  (bind _returnvalue_7 (Transformation|GetWorldLocation _cinecamera_3))
  (bind _returnvalue_8 (Transformation|GetWorldRotation _cinecamera_3))
  (bind _returnvalue_9 (Transformation|GetWorldLocation _cinecamera_6))
  (bind _returnvalue_10 (Transformation|GetWorldRotation _cinecamera_6))
  (bind _returnvalue_11 (Transformation|GetWorldLocation _cinecamera_5))
  (bind _returnvalue_12 (Transformation|GetWorldRotation _cinecamera_5))
  (bind _moving (Timeline|Timeline_0 PlayFromStart)
    (:Update
      (switch Utilities|FlowControl|Switch|SwitchonE_MainMenuOptions ReturnMainMenu
        (:NewEnumerator0
          (Transformation|SetWorldLocationAndRotation _cinecamera_5 (Math|Vector|MakeVector (.x _returnvalue_11) (.y _returnvalue_11) (Math|Float|Lerp (.z _returnvalue_11) Location _moving)) (Math|Rotator|MakeRotator (.roll _returnvalue_12) (Math|Float|Lerp (.pitch _returnvalue_12) Rotation _moving) (.yaw _returnvalue_12)) false false :!pinned true) ; Play
        )
        (:NewEnumerator1
          (Transformation|SetWorldLocationAndRotation _cinecamera_3 (Math|Vector|MakeVector (Math|Float|Lerp (.x _returnvalue_7) Location _moving) (.y _returnvalue_7) (.z _returnvalue_7)) (Math|Rotator|MakeRotator (.roll _returnvalue_8) (.pitch _returnvalue_8) (Math|Float|Lerp (.yaw _returnvalue_8) Rotation _moving)) false false :!pinned true) ; Game
        )
        (:NewEnumerator2
          (Transformation|SetWorldLocationAndRotation _cinecamera_6 (Math|Vector|MakeVector (Math|Float|Lerp (.x _returnvalue_9) Location _moving) (.y _returnvalue_9) (.z _returnvalue_9)) (Math|Rotator|MakeRotator (.roll _returnvalue_10) (.pitch _returnvalue_10) (Math|Float|Lerp (.yaw _returnvalue_10) Rotation _moving)) false false :!pinned true) ; Video
        )
        (:NewEnumerator3
          (Transformation|SetWorldLocationAndRotation _cinecamera_4 (Math|Vector|MakeVector (.x _returnvalue_5) (.y _returnvalue_5) (Math|Float|Lerp (.z _returnvalue_5) Location _moving)) (Math|Rotator|MakeRotator (Math|Float|Lerp (.roll _returnvalue_6) Rotation _moving) (.pitch _returnvalue_6) (.yaw _returnvalue_6)) false false :!pinned true) ; Audio
        )
        (:NewEnumerator5
          (Transformation|SetWorldLocationAndRotation _cinecamera_2 (Math|Vector|MakeVector (.x _returnvalue_3) (.y _returnvalue_3) (Math|Float|Lerp (.z _returnvalue_3) Location _moving)) (Math|Rotator|MakeRotator (.roll _returnvalue_4) (.pitch _returnvalue_4) (Math|Float|Lerp (.yaw _returnvalue_4) Rotation _moving)) false false :!pinned true) ; Extras
        )
        (:NewEnumerator6
          (Transformation|SetWorldLocationAndRotation _cinecamera (Math|Vector|MakeVector (Math|Float|Lerp (.x _returnvalue) Location _moving) (.y _returnvalue) (.z _returnvalue)) (Math|Rotator|MakeRotator (.roll _returnvalue_2) (.pitch _returnvalue_2) (Math|Float|Lerp (.yaw _returnvalue_2) Rotation _moving)) false false :!pinned true) ; Exit
        )))))

(fn ConstructionScript)